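; Actor component implementing a small feedforward neural network with a fitness score that grows over time while Alive, suited to neuroevolution.
; Neurons live in a map keyed by layer and index, each holding a value and random incoming weights, with no biases.
; FeedForward injects inputs, propagates weighted sums through a sigmoid layer by layer, and returns the last layer.
; MutateNetwork re-randomizes individual weights by threshold probability.
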(event EventTick
  (params (DeltaSeconds :type Float%20%28single-precision%29))
  (if (Variables|Default|GetAlive)
    (CallFunction|AddFitness (* DeltaSeconds 15.0))))

(fn InitializeNetwork
  (params (NeuralLayers :type Array%20of%20Integers))
  (Variables|Default|SetNeuralLayers NeuralLayers)
  (CallFunction|InitializeNeurons))

(fn InitializeNeurons
  (bind _tempweights (LocalVariables|GetTempWeights))
  (for (_array_element _array_index) (Variables|Default|GetNeuralLayers)
    (for _index (range 0 (- _array_element 1))
      (if (> _array_index 0)
        (Utilities|Array|Resize (LocalVariables|GetTempWeights) (CallFunction|GetSizePreviousLayer _array_index))
        (for (_ _array_index_2) _tempweights
          (Utilities|Array|SetArrayElem _tempweights _array_index_2 (Math|Random|RandomFloatinRange -1.0 1.0)))
        (Utilities|Map|Add (Variables|Default|GetNeurons) (Utilities|Struct|MakeStruct_Coord _array_index _index) (Utilities|Struct|MakeStruct_Neuron 0.0 (LocalVariables|GetTempWeights)))
        (else
          (Utilities|Map|Add (Variables|Default|GetNeurons) (Utilities|Struct|MakeStruct_Coord _array_index _index) (Utilities|Struct|MakeStruct_Neuron 0.0 0)))))))

(fn GetSizePreviousLayer
  (params (CurrentLayer :type Integer))
  (return (Utilities|Array|Get(acopy) (Variables|Default|GetNeuralLayers) (- CurrentLayer 1))))

(fn InjectInputs
  (params (Inputs :type Array%20of%20Floats%20%28double-precision%29))
  (bind _neurons (Variables|Default|GetNeurons))
  (for (_array_element _array_index) Inputs
    (Utilities|Map|Add _neurons (Utilities|Struct|MakeStruct_Coord 0 _array_index) (Utilities|Struct|MakeStruct_Neuron _array_element (.weights (.Value (Utilities|Map|Find _neurons (Utilities|Struct|MakeStruct_Coord 0 _array_index))))))))

(fn GetOutputs
  (bind _neurallayers (Variables|Default|GetNeuralLayers))
  (bind _returnvalue (Utilities|Array|LastIndex _neurallayers))
  (for _index (range 0 (- (Utilities|Array|Get(acopy) _neurallayers _returnvalue) 1))
    (Utilities|Array|Add (LocalVariables|GetTempOutputs) (.value (.Value (Utilities|Map|Find (Variables|Default|GetNeurons) (Utilities|Struct|MakeStruct_Coord _returnvalue _index))))))
  (return (LocalVariables|GetTempOutputs)))

(fn FeedForward
  (params (Inputs :type Array%20of%20Floats%20%28double-precision%29))
  (CallFunction|InjectInputs Inputs)
  (for _index (range 1 (Utilities|Array|LastIndex (Variables|Default|GetNeuralLayers)))
    (CallFunction|FeedLayer _index))
  (return (CallFunction|GetOutputs)))

(fn FeedNeuron
  (params (CoordNeuron :type Struct%20Coord%20Structure))
  (for (_array_element _array_index) (.weights (.Value (Utilities|Map|Find (Variables|Default|GetNeurons) (Utilities|Struct|MakeStruct_Coord (.x CoordNeuron) (.y CoordNeuron)))))
    (LocalVariables|SetTempValue (+ (LocalVariables|GetTempValue) (* _array_element (.value (.Value (Utilities|Map|Find (Variables|Default|GetNeurons) (Utilities|Struct|MakeStruct_Coord (- (.x CoordNeuron) 1) _array_index))))))))
  (Utilities|Map|Add (Variables|Default|GetNeurons) (Utilities|Struct|MakeStruct_Coord (.x CoordNeuron) (.y CoordNeuron)) (Utilities|Struct|MakeStruct_Neuron (CallFunction|Sigmoid (LocalVariables|GetTempValue)) (.weights (.Value (Utilities|Map|Find (Variables|Default|GetNeurons) (Utilities|Struct|MakeStruct_Coord (.x CoordNeuron) (.y CoordNeuron))))))))

(fn Sigmoid
  (params (Value :type Float%20%28double-precision%29))
  (return (|(1/(1+(e((0-x))))) Value)))

(fn FeedLayer
  (params (Layer :type Integer))
  (for _index (range 0 (- (Utilities|Array|Get(acopy) (Variables|Default|GetNeuralLayers) Layer) 1))
    (CallFunction|FeedNeuron (Utilities|Struct|MakeStruct_Coord Layer _index))))

(fn AddFitness
  (params (FitnessToAdd :type Float%20%28double-precision%29))
  (Variables|Default|SetFitness (+ (Variables|Default|GetFitness) FitnessToAdd)))

(fn MutateWeight
  (params (X :type Integer) (Y :type Integer) (IndexWeight :type Integer) (Threshold :type Float%20%28double-precision%29))
  (bind _neurons (Variables|Default|GetNeurons))
  (bind _value (Utilities|Map|Find _neurons (Utilities|Struct|MakeStruct_Coord X Y)))
  (if (< (Math|Random|RandomFloat) Threshold)
    (bind _output_get (LocalVariables|SetTempWeights (.weights _value)))
    (Utilities|Array|SetArrayElem _output_get IndexWeight (Math|Random|RandomFloatinRange -1.0 1.0))
    (Utilities|Map|Add _neurons (Utilities|Struct|MakeStruct_Coord X Y) (Utilities|Struct|MakeStruct_Neuron (.value _value) (LocalVariables|GetTempWeights)))))

(fn MutateNeuron
  (params (X :type Integer) (Y :type Integer) (Threshold :type Float%20%28double-precision%29))
  (for _index (range 0 (Utilities|Array|LastIndex (.weights (.Value (Utilities|Map|Find (Variables|Default|GetNeurons) (Utilities|Struct|MakeStruct_Coord X Y))))))
    (CallFunction|MutateWeight X Y _index Threshold)))

(fn MutateLayer
  (params (X :type Integer) (Threshold :type Float%20%28double-precision%29))
  (for _index (range 0 (- (Utilities|Array|Get(acopy) (Variables|Default|GetNeuralLayers) X) 1))
    (CallFunction|MutateNeuron X _index Threshold)))

(fn MutateNetwork
  (params (Threshold :type Float%20%28double-precision%29))
  (for _index (range 0 (Utilities|Array|LastIndex (Variables|Default|GetNeuralLayers)))
    (CallFunction|MutateLayer _index Threshold)))